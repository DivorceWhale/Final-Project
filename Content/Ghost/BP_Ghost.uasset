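; Pac-Man style ghost enemy that roams, chases the player, and can be eaten while scared.
; Roaming starts after a delay and loops through random reachable points; Tick and pawn sensing drive chasing, falling back to roaming.
; When IsScared, it changes walk speed and moves to the raw player-to-ghost offset vector as its flee destination.
; Player overlap either destroys the scared ghost for points or costs a life and triggers PacManDeath.
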(event `self.ReceiveBeginPlay`
  (`KismetSystemLibrary.Delay` 5.0)
  (`self.Random Roam`))

(event `Random Roam`
  ; Random Roam
  (`|AIMoveTo` self (`NavigationSystemV1.K2_GetRandomReachablePointInRadius` (`self.K2_GetActorLocation`) 3000.0 null null) null
    (:`OnSuccess`
      _)
    (:`OnFail`
      _))
  (`self.Random Roam`))

(event `self.ReceiveTick`
  (params (DeltaSeconds :type "Float (single-precision)"))
  (bind _returnvalue (`GameplayStatics.GetPlayerCharacter` 0))
  ; Ghost Movement
  (bind _asbp_third_person_character (cast `/Game/ThirdPerson/Blueprints/BP_ThirdPersonCharacter` _returnvalue :!label _label))
  (if (`self.IsScared`)
    (set `CharacterMovementComponent.MaxWalkSpeed` 400.0 (`self.CharacterMovement`))
    (`|AIMoveTo` self (* (- (`self.K2_GetActorLocation`) (`self.K2_GetActorLocation` _returnvalue)) 1.0) null)
    (else
      (`|AIMoveTo` self (0.0 0.0 0.0) _asbp_third_person_character
        (:`OnFail`
          (`KismetSystemLibrary.RetriggerableDelay` 3.0)
          (`self.Random Roam` :!label _label_2))))))

(event `self.PawnSensing.OnSeePawn`
  (params (Pawn :type "Pawn Object Reference"))
  ; Ghost Movement
  (if (`self.ChasePlayer`)
    (goto _label)
    (else
      (goto _label_2))))

(event `self.Attack Collider.OnComponentBeginOverlap`
  (params (OverlappedComponent :type "PrimitiveComponent Object Reference") (OtherActor :type "Actor Object Reference") (OtherComp :type "PrimitiveComponent Object Reference") (OtherBodyIndex :type Integer) (bFromSweep :type Boolean) (SweepResult :type "HitResult Structure (by ref)"))
  (bind _third_person_character (`self.Third Person Character`))
  ; Scared Mode Point
  (bind _asbp_third_person_character (cast `/Game/ThirdPerson/Blueprints/BP_ThirdPersonCharacter` OtherActor))
  (bind _output_get (set `self.Third Person Character` _asbp_third_person_character))
  (if (`self.IsScared`)
    (`self.K2_DestroyActor`)
    (set `/Game/ThirdPerson/Blueprints/BP_ThirdPersonCharacter.PelletScore` (+ (`/Game/ThirdPerson/Blueprints/BP_ThirdPersonCharacter.PelletScore` _third_person_character) 1000) _third_person_character)
    (else
      (set `/Game/ThirdPerson/Blueprints/BP_ThirdPersonCharacter.Lives` (- (`/Game/ThirdPerson/Blueprints/BP_ThirdPersonCharacter.Lives` _output_get) 1) _output_get)
      (`/Game/ThirdPerson/Blueprints/BP_ThirdPersonCharacter.PacMan Death` (`self.Third Person Character`)))))

(fn `UserConstructionScript`)