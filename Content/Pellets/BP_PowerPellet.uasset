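; Power pellet pickup that flashes in the level and puts the game into scared mode when collected.
; Overlap by the third-person character adds to its pellet score, plays a sound, calls ActivateScaredMode on the game mode found via GetAllActorsOfClass, then destroys the pellet.
; Flashing toggles mesh visibility with delays behind a DoOnce, triggered from BeginPlay and Tick and reset after each blink.
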(event `self.ReceiveBeginPlay`
  (`self.Flashing`))

(event `self.PelletPU trigger.OnComponentBeginOverlap`
  (params (OverlappedComponent :type "PrimitiveComponent Object Reference") (OtherActor :type "Actor Object Reference") (OtherComp :type "PrimitiveComponent Object Reference") (OtherBodyIndex :type Integer) (bFromSweep :type Boolean) (SweepResult :type "HitResult Structure (by ref)"))
  ; Points
  (bind _asbp_third_person_character (cast `/Game/ThirdPerson/Blueprints/BP_ThirdPersonCharacter` OtherActor))
  (set `/Game/ThirdPerson/Blueprints/BP_ThirdPersonCharacter.PelletScore` (+ (`/Game/ThirdPerson/Blueprints/BP_ThirdPersonCharacter.PelletScore` _asbp_third_person_character) 100) _asbp_third_person_character)
  (`GameplayStatics.PlaySound2D` "/Game/audio/pelletwav.pelletwav" 1.0 1.0 0.0 null null)
  (bind _outactors (`GameplayStatics.GetAllActorsOfClass` "/Game/ThirdPerson/Blueprints/BP_ThirdPersonGameMode.BP_ThirdPersonGameMode_C"))
  (`/Game/ThirdPerson/Blueprints/BP_ThirdPersonGameMode.Activate Scared Mode` _outactors)
  (`self.K2_DestroyActor`))

(event `self.ReceiveTick`
  (params (DeltaSeconds :type "Float (single-precision)"))
  ; Flashing
  (`/Engine/EditorBlueprintResources/StandardMacros.DoOnce` false :!label _label
    (:`Completed`
      (`SceneComponent.SetVisibility` (`self.Pellet`) false false)
      (`KismetSystemLibrary.Delay` 0.5)
      (`SceneComponent.SetVisibility` (`self.Pellet`) true false)
      (`KismetSystemLibrary.Delay` 0.5)
      (goto _label :!via `Reset`))))

(event `Flashing`
  ; Flashing
  (goto _label))

(fn `UserConstructionScript`)